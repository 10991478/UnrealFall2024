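; Base countdown timer that kills the third-person player character when time runs out.
; Unpausing runs a delayed while loop that decrements once per second, while pausing stops it and hides the display.
; Event dispatchers broadcast visibility and formatted minutes:seconds text to listeners.
; On expiry it resets and subtracts the player's max health, and it also resets whenever the player's death dispatcher fires.
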(event `self.ReceiveBeginPlay`
  (bind _output_get (set `self.TotalInitialTime` (+ (* (`self.InitialMinutes`) 60) (`self.InitialSeconds`))))
  (set `self.TotalCurrentTime` _output_get)
  (bind _asbp_third_person_character (cast `/Game/ThirdPerson/Blueprints/BP_ThirdPersonCharacter` (`Controller.K2_GetPawn` (`GameplayStatics.GetPlayerController` 0))))
  (bind _output_get_2 (set `self.PlayerRef` _asbp_third_person_character))
  (add `/Game/ThirdPerson/Blueprints/BP_ThirdPersonCharacter.ED_PlayerDied` _output_get_2 (delegate `PlayerDied`)))

(event `UnpauseTimer`
  (bind _playerref (`self.PlayerRef`))
  (`self.ED_SetTimerVisibility` true)
  (if (and (> (`self.TotalCurrentTime`) 0) (not (`self.TimerIsRunning`)))
    (set `self.TimerUnpaused` true)
    (`/Game/Blueprints/Macros/BML_BreakAndDelay_Actor.WhileLoopWithDelay` (`self.TimerUnpaused`) 1.0
      (:`LoopBody`
        (bind _timerranout (`self.DecrementSeconds`))
        (if _timerranout
          (`self.ResetTimer`)
          (`/Game/ThirdPerson/Blueprints/BP_ThirdPersonCharacter.SubtractFromHealth` _playerref (`/Game/ThirdPerson/Blueprints/BP_ThirdPersonCharacter.MaxHealth` _playerref)))))))

(event `PauseTimer`
  (set `self.TimerUnpaused` false)
  (`self.ED_SetTimerVisibility` false))

(event `ResetTimer`
  (bind _output_get (set `self.TotalCurrentTime` (`self.TotalInitialTime`)))
  (bind (_minutes _seconds) (`self.CalculateTimeInMinutesAndSeconds` _output_get))
  (bind _output_get_2 (set `self.DisplayTime` (`|FormatText` "{min} : {sec}" (`KismetTextLibrary.Conv_IntToText` _minutes false true 2 2) (`KismetTextLibrary.Conv_IntToText` _seconds false true 2 2))))
  (`self.ED_UpdateCurrentTimer` _output_get_2))

(event `PlayerDied`
  (`self.ResetTimer`))

(fn `CalculateTimeInMinutesAndSeconds`
  (params (InputTime :type Integer))
  (returns (Minutes :type Integer) (Seconds :type Integer))
  (bind _returnvalue (mod InputTime 60))
  (return (/ (- InputTime _returnvalue) 60) _returnvalue))

(fn `DecrementSeconds`
  (returns (TimerRanOut :type Boolean))
  (bind _displaytime (`self.DisplayTime`))
  (bind _returnvalue (- (`self.TotalCurrentTime`) 1))
  (if (> _returnvalue 0)
    (bind _output_get (set `self.TotalCurrentTime` _returnvalue))
    (bind (_minutes _seconds) (`self.CalculateTimeInMinutesAndSeconds` _output_get))
    (set `self.DisplayTime` (`|FormatText` "{min} : {sec}" (`KismetTextLibrary.Conv_IntToText` _minutes false true 2 2) (`KismetTextLibrary.Conv_IntToText` _seconds false true 2 2)))
    (else
      (set `self.TotalCurrentTime` 0)
      (set `self.DisplayTime` "00 : 00")
      (set `self.TimerUnpaused` false)))
  (`self.ED_UpdateCurrentTimer` _displaytime)
  (`KismetSystemLibrary.PrintText` _displaytime)
  (return (not (`self.TimerUnpaused`))))

(fn `UserConstructionScript`)