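; BP_TimerDisplayHandler shows countdown timer text on screen through a single WB_TimerDisplay widget.
; On BeginPlay it creates the widget for the first player, adds it to the viewport hidden, and binds to each CountdownTimers entry's update and visibility event dispatchers.
; Those dispatchers drive the widget's text and show or hide it, so all listed timers share one display.
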(event `self.ReceiveBeginPlay`
  (bind _returnvalue (`|CreateWidget` "/Game/Blueprints/Timers/WB_TimerDisplay.WB_TimerDisplay_C" (`GameplayStatics.GetPlayerController` 0)))
  (bind _output_get (set `self.TimerWidgetRef` _returnvalue))
  (`UserWidget.AddToViewport` _output_get 0)
  (`Widget.SetVisibility` _output_get "Hidden")
  (for _array_element (`self.CountdownTimers`)
    (add `/Game/Blueprints/Timers/BP_Base_CountdownTimer.ED_UpdateCurrentTimer` _array_element (delegate `UpdateTimer`))
    (add `/Game/Blueprints/Timers/BP_Base_CountdownTimer.ED_SetTimerVisibility` _array_element (delegate `SetVisibility`))))

(event `UpdateTimer`
  (params (`Display Text` :type Text))
  (`/Game/Blueprints/Timers/WB_TimerDisplay.SetTimerText` (`self.TimerWidgetRef`) `Display Text`))

(event `SetVisibility`
  (params (IsVisible :type Boolean))
  (bind _timerwidgetref (`self.TimerWidgetRef`))
  (if IsVisible
    (`Widget.SetVisibility` _timerwidgetref "Visible")
    (else
      (`Widget.SetVisibility` _timerwidgetref "Hidden"))))

(fn `UserConstructionScript`)