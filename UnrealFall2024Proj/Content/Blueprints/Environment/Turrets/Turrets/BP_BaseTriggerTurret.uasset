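; Base trigger turret that fires repeatedly while actors of accepted classes are inside its box collider.
; Overlap events filter actors against a class list, then adjust a zero-clamped counter that sets the overlapped flag.
; Each qualifying entry calls the shooting loop after an initial delay.
; The loop calls ShootBullet and waits between shots, repeating until the flag clears.
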(event `self.ReceiveBeginPlay`
  (`parent.ReceiveBeginPlay`)
  (set `self.CurrentlyOverlapped` false)
  (set `self.NumOfCurrentOverlaps` 0))

(event `ShootingLoop`
  (if (`self.CurrentlyOverlapped`) :!label _label
    (`self.ShootBullet`)
    (`KismetSystemLibrary.Delay` (`self.TimeBetweenShots`))
    (goto _label)))

(event `self.BoxCollider.OnComponentBeginOverlap`
  (params (OverlappedComponent :type "PrimitiveComponent Object Reference") (OtherActor :type "Actor Object Reference") (OtherComp :type "PrimitiveComponent Object Reference") (OtherBodyIndex :type Integer) (bFromSweep :type Boolean) (SweepResult :type "HitResult Structure (by ref)"))
  (bind _successfulcast (`self.CastActorToAcceptableOverlapClasses` OtherActor))
  (if _successfulcast
    (`self.UpdateCurrentlyOverlapped` false)
    (`KismetSystemLibrary.Delay` (`self.InitialDelay`))
    (`self.ShootingLoop`)))

(event `self.BoxCollider.OnComponentEndOverlap`
  (params (OverlappedComponent :type "PrimitiveComponent Object Reference") (OtherActor :type "Actor Object Reference") (OtherComp :type "PrimitiveComponent Object Reference") (OtherBodyIndex :type Integer))
  (bind _successfulcast (`self.CastActorToAcceptableOverlapClasses` OtherActor))
  (if _successfulcast
    (`self.UpdateCurrentlyOverlapped` true)))

(fn `CastActorToAcceptableOverlapClasses`
  (params (Actor :type "Actor Object Reference"))
  (returns (SuccessfulCast :type Boolean))
  (locals (ActorPassesCast :type Boolean))
  (set `local.ActorPassesCast` false)
  (for _array_element (`self.AcceptableOverlapClasses`)
    (if (`KismetMathLibrary.ClassIsChildOf` (`GameplayStatics.GetObjectClass` Actor) _array_element)
      (set `local.ActorPassesCast` true)
      (break)))
  (return (`local.ActorPassesCast`)))

(fn `UpdateCurrentlyOverlapped`
  (params (Subtract :type Boolean))
  (returns (CurrentlyOverlapping :type Boolean))
  (bind _returnvalue (+ (`KismetMathLibrary.SelectInt` -1 1 Subtract) (`self.NumOfCurrentOverlaps`)))
  (if (<= _returnvalue 0)
    (set `self.NumOfCurrentOverlaps` 0)
    (bind _output_get (set `self.CurrentlyOverlapped` false))
    (return _output_get)
    (else
      (set `self.NumOfCurrentOverlaps` _returnvalue)
      (bind _output_get_2 (set `self.CurrentlyOverlapped` true))
      (return _output_get_2))))

(fn `UserConstructionScript`
  (`parent.UserConstructionScript`))