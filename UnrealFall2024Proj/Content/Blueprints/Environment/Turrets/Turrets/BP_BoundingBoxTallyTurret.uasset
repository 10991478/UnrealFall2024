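; Turret that fires on a timer while enabled and the player character is inside its BoundingBox, with a starting offset delaying the first shot.
; Each shot adds to the BoundingBox's tally, which is broadcast back through a bound dispatcher alongside the begin and end overlap events.
; The tally is checked against two thresholds in sequence; breaking either advances the stage and sets the turret enabled.
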(event `self.ReceiveTick`
  (params (DeltaSeconds :type "Float (single-precision)"))
  (bind _timesincelastshot (`self.TimeSinceLastShot`))
  (if (and (`self.PlayerIsWithinBounds`) (`self.CurrentlyEnabled`))
    (if (>= _timesincelastshot (`self.TimeBetweenShots`))
      (`self.ShootBullet` true)
      (set `self.TimeSinceLastShot` 0.0)
      (`/Game/Blueprints/Environment/BoxTriggers/BP_Base_BoxTriggerWithTally.AddToTally` (`self.BoundingBox`) 1)
      (else
        (set `self.TimeSinceLastShot` (+ _timesincelastshot DeltaSeconds))))))

(event `self.ReceiveBeginPlay`
  (bind _boundingbox (`self.BoundingBox`))
  (`parent.ReceiveBeginPlay`)
  (set `self.PlayerIsWithinBounds` false)
  (bind _asbp_third_person_character (cast `/Game/ThirdPerson/Blueprints/BP_ThirdPersonCharacter` (`GameplayStatics.GetPlayerCharacter` 0)))
  (set `self.PlayerCharacter` _asbp_third_person_character)
  (add `/Game/Blueprints/Environment/BoxTriggers/BP_Base_BoxTrigger.ED_BeginOverlap` _boundingbox (delegate `/Game/Blueprints/BlueprintInterfaces/TriggerBoxReaction.BeginOverlapFunc`))
  (add `/Game/Blueprints/Environment/BoxTriggers/BP_Base_BoxTrigger.ED_EndOverlap` _boundingbox (delegate `/Game/Blueprints/BlueprintInterfaces/TriggerBoxReaction.EndOverlapFunc`))
  (add `/Game/Blueprints/Environment/BoxTriggers/BP_Base_BoxTriggerWithTally.ED_BroadcastTally` _boundingbox (delegate `CurrentTallyUpdated`))
  (set `self.TimeSinceLastShot` (* (`self.StartingTimeOffset`) -1.0)))

(event `/Game/Blueprints/BlueprintInterfaces/TriggerBoxReaction.BeginOverlapFunc`
  (params (OtherActor :type "Actor Object Reference"))
  (cast `/Game/ThirdPerson/Blueprints/BP_ThirdPersonCharacter` OtherActor)
  (set `self.PlayerIsWithinBounds` true))

(event `/Game/Blueprints/BlueprintInterfaces/TriggerBoxReaction.EndOverlapFunc`
  (params (OtherActor :type "Actor Object Reference"))
  (cast `/Game/ThirdPerson/Blueprints/BP_ThirdPersonCharacter` OtherActor)
  (set `self.PlayerIsWithinBounds` false))

(event `CurrentTallyUpdated`
  (params (CurrentTally :type Integer))
  (bind _returnvalue (select `int` (`self.ThreshholdsBroken`) :`0` (`self.EventThreshhold_01`) :`1` (`self.EventThreshhold_02`) :`2` -1))
  (if (== _returnvalue -1)
    _
    (elif (>= CurrentTally _returnvalue)
      (if (select `int` (`self.ThreshholdsBroken`) :`0` true :`1` false)
        (`self.BrokeFirstThreshhold`)
        (else
          (`self.BrokeSecondThreshhold`))))))

(event `BrokeFirstThreshhold`
  (`/Engine/EditorBlueprintResources/StandardMacros.IncrementInt` (`self.ThreshholdsBroken`)
    (:`  `
      (set `self.CurrentlyEnabled` true)
      (`KismetSystemLibrary.PrintString` "Homing Turret reached first threshhold"))))

(event `BrokeSecondThreshhold`
  (`/Engine/EditorBlueprintResources/StandardMacros.IncrementInt` (`self.ThreshholdsBroken`)
    (:`  `
      (set `self.CurrentlyEnabled` true))))

(fn `UserConstructionScript`
  (`parent.UserConstructionScript`))