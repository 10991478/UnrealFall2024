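; A hidden platform actor that appears and moves to a raised position once a tally reaches a threshold.
; BeginPlay hides the platform and binds to the tally broadcast from BoundingBox.
; When the threshold is met, the platform becomes visible and Tick lerps it from its current location toward RaisedPos, giving an ease-out motion.
; Movement stops permanently once the platform is within an acceptable distance of that target.
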(event `self.ReceiveBeginPlay`
  (add `/Game/Blueprints/Environment/BoxTriggers/BP_Base_BoxTriggerWithTally.ED_BroadcastTally` (`self.BoundingBox`) (delegate `CurrentTallyUpdated`))
  (`SceneComponent.SetVisibility` (`self.Platform`) false false))

(event `CurrentTallyUpdated`
  (params (CurrentTally :type Integer))
  (if (and (>= CurrentTally (`self.EventThreshhold`)) (`self.HasNotYetMoved`))
    (set `self.MovementEnabled` true)
    (`SceneComponent.SetVisibility` (`self.Platform`) true false)))

(event `self.ReceiveTick`
  (params (DeltaSeconds :type "Float (single-precision)"))
  (if (and (`self.MovementEnabled`) (`self.HasNotYetMoved`))
    (bind _disttolocation (`self.LerpToRaisedLocation` (* DeltaSeconds (`self.LerpRate`))))
    (if (<= _disttolocation (`self.AcceptableDistanceToRaisedPos`))
      (set `self.HasNotYetMoved` false))))

(fn `LerpToRaisedLocation`
  (params (LerpRate :type "Float (double-precision)"))
  (returns (DistToLocation :type "Float (double-precision)"))
  (bind _platform (`self.Platform`))
  (bind _returnvalue (`SceneComponent.K2_GetComponentLocation` (`self.RaisedPos`)))
  (bind _returnvalue_2 (`KismetMathLibrary.VLerp` (`SceneComponent.K2_GetComponentLocation` _platform) _returnvalue LerpRate))
  (`SceneComponent.K2_SetWorldLocation` _platform _returnvalue_2 false false)
  (return (`KismetMathLibrary.Vector_Distance` _returnvalue_2 _returnvalue)))

(fn `UserConstructionScript`)