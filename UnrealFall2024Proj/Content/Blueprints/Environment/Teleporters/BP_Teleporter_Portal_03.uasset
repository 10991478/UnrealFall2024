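; BP_Teleporter_Portal_03 is a portal actor that teleports the third-person character from its collider to an exit point.
; On overlap while active, it plays a sound at the exit, waits a teleportation delay, then moves the character there with zero rotation.
; An active flag clears after the teleport and resets after an activation delay, serving as a cooldown that does not cover the initial wait.
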(event `self.ReceiveBeginPlay`
  (set `self.TeleportersAreActive` true))

(event `self.Teleporter_01_Collider.OnComponentBeginOverlap`
  (params (OverlappedComponent :type "PrimitiveComponent Object Reference") (OtherActor :type "Actor Object Reference") (OtherComp :type "PrimitiveComponent Object Reference") (OtherBodyIndex :type Integer) (bFromSweep :type Boolean) (SweepResult :type "HitResult Structure (by ref)"))
  (if (`self.TeleportersAreActive`)
    (bind _asbp_third_person_character (cast `/Game/ThirdPerson/Blueprints/BP_ThirdPersonCharacter` OtherActor))
    (`GameplayStatics.PlaySoundAtLocation` "/Game/Audio/SoundEffects/game-teleport-90735.game-teleport-90735" (`SceneComponent.K2_GetComponentLocation` (`self.Teleporter_01_Exit`)) (struct) 1.0 1.0 0.0 null null null null)
    (`KismetSystemLibrary.Delay` (`self.TeleportationDelay`))
    (`self.K2_TeleportTo` :`self` _asbp_third_person_character :`DestLocation` (`SceneComponent.K2_GetComponentLocation` (`self.Teleporter_01_Exit`)))
    (set `self.TeleportersAreActive` false)
    (`KismetSystemLibrary.Delay` (`self.ActivationDelay`))
    (set `self.TeleportersAreActive` true)))

(fn `UserConstructionScript`)