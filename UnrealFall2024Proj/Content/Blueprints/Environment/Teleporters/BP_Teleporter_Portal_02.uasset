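; Timed teleporter portal that sends the third-person character to the location of its linked TeleporterExit, with rotation zeroed.
; BeginPlay applies the StartsActive state, then Tick uses latent Delays for an initial wait and alternating on/off periods.
; ChangeActivity keeps collider activation, portal visibility and the active flag together.
; Overlaps teleport only while active, and switching on also teleports characters already inside the collider.
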(event `self.ReceiveBeginPlay`
  ;[1 1 1] Setting Teleporter Activity at Start
  (set `self.InitialDelayIsDone` false)
  (bind _output_get (set `self.TeleporterIsActive` (`self.StartsActive`)))
  (if _output_get
    (`ActorComponent.SetActive` (`self.Teleporter_Collider`) true false)
    (`SceneComponent.SetVisibility` (`self.Teleporter`) true false)
    (else
      (`ActorComponent.SetActive` (`self.Teleporter_Collider`) false false)
      (`SceneComponent.SetVisibility` (`self.Teleporter`) false false))))

(event `self.ReceiveTick`
  (params (DeltaSeconds :type "Float (single-precision)"))
  ;[1 1 1] Setting Visibile/Invisible and Active/Inactive
  (if (not (`self.InitialDelayIsDone`))
    (`KismetSystemLibrary.Delay` (`self.InitialDelay`))
    (set `self.InitialDelayIsDone` true))
  (if (`self.TeleporterIsActive`)
    (`KismetSystemLibrary.Delay` (`self.TimeOn`))
    (`self.ChangeActivity` false)
    (else
      (`KismetSystemLibrary.Delay` (`self.TimeOff`))
      (`self.ChangeActivity` true)
      (for _array_element (`PrimitiveComponent.GetOverlappingActors` (`self.Teleporter_Collider`) "/Game/ThirdPerson/Blueprints/BP_ThirdPersonCharacter.BP_ThirdPersonCharacter_C")
        (`self.Teleport Player` _array_element)))))

(event `self.Teleporter_Collider.OnComponentBeginOverlap`
  (params (OverlappedComponent :type "PrimitiveComponent Object Reference") (OtherActor :type "Actor Object Reference") (OtherComp :type "PrimitiveComponent Object Reference") (OtherBodyIndex :type Integer) (bFromSweep :type Boolean) (SweepResult :type "HitResult Structure (by ref)"))
  ;[1 1 1] Detecting Collisions and teleporting
  (`self.Teleport Player` OtherActor))

(fn `ChangeActivity`
  (params (SetActive :type Boolean))
  (`ActorComponent.SetActive` (`self.Teleporter_Collider`) SetActive false)
  (`SceneComponent.SetVisibility` (`self.Teleporter`) SetActive false)
  (set `self.TeleporterIsActive` SetActive))

(fn `Teleport Player`
  (params (PlayerActor :type "Actor Object Reference"))
  (if (`self.TeleporterIsActive`)
    (bind _asbp_third_person_character (cast `/Game/ThirdPerson/Blueprints/BP_ThirdPersonCharacter` PlayerActor))
    (`self.K2_TeleportTo` :`self` _asbp_third_person_character :`DestLocation` (`SceneComponent.K2_GetComponentLocation` (`Actor.RootComponent` (`self.TeleporterExit`))))))

(fn `UserConstructionScript`)