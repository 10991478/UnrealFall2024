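; Base Blueprint for a trigger-driven door that opens when enough triggers are active.
; Add and remove functions adjust the active trigger count, which resets on BeginPlay, and compare it to TriggerThreshold to call open or close.
; Removing more than the current count zeroes it and returns true without calling close.
; The Open_Door and Close_Door events are empty here.
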(event `self.ReceiveBeginPlay`
  (set `self.CurrentlyActivatedTriggers` 0))

(event `Open_Door`)

(event `Close_Door`)

(fn `AddActiveTriggers`
  (params (AddAmount :type Integer))
  (returns (AmountReachesThreshold :type Boolean))
  (bind _output_get (set `self.CurrentlyActivatedTriggers` (+ AddAmount (`self.CurrentlyActivatedTriggers`))))
  (bind _satisfy (`self.CurrentTriggersSatisfyThreshold`))
  (if _satisfy
    (`self.Open_Door`))
  (return (>= _output_get (`self.TriggerThreshold`))))

(fn `CurrentTriggersSatisfyThreshold`
  (returns (Satisfy :type Boolean))
  (if (>= (`self.CurrentlyActivatedTriggers`) (`self.TriggerThreshold`))
    (return true)
    (else
      (return false))))

(fn `RemoveActiveTriggers`
  (params (RemoveAmount :type Integer))
  (returns (DippedBelowZero :type Boolean))
  (bind _returnvalue (- (`self.CurrentlyActivatedTriggers`) RemoveAmount))
  (if (>= _returnvalue 0)
    (set `self.CurrentlyActivatedTriggers` _returnvalue)
    (bind _satisfy (`self.CurrentTriggersSatisfyThreshold`))
    (if (not _satisfy)
      (`self.Close_Door`))
    (return false)
    (else
      (set `self.CurrentlyActivatedTriggers` 0)
      (return true))))

(fn `UserConstructionScript`)