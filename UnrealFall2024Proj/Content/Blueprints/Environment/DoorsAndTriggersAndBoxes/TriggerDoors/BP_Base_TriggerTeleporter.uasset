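; Trigger-driven teleporter that reuses its parent's OpenDoor and CloseDoor events to switch on and off, toggling the collider and teleporter visibility.
; While active, it sends overlapping objects of allowed classes to TeleporterExit, including those already inside when it opens.
; Actors teleport with zeroed rotation, and an overlapping static mesh component that also passes the class check is moved separately.
; BeginPlay refreshes the trigger state through zero-value add and remove calls.
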(event `self.ReceiveBeginPlay`
  (`parent.ReceiveBeginPlay`)
  (`self.RemoveActiveTriggers` 0)
  (`self.AddActiveTriggers` 0))

(event `self.TeleporterCollider.OnComponentBeginOverlap`
  (params (OverlappedComponent :type "PrimitiveComponent Object Reference") (OtherActor :type "Actor Object Reference") (OtherComp :type "PrimitiveComponent Object Reference") (OtherBodyIndex :type Integer) (bFromSweep :type Boolean) (SweepResult :type "HitResult Structure (by ref)"))
  (bind _successfulcast (`self.CastObjectToAcceptableOverlapClasses` OtherActor))
  (if _successfulcast
    (`self.TeleportObject` OtherActor)
    (bind _successfulcast_2 (`self.CastObjectToAcceptableOverlapClasses` OtherComp))
    (if _successfulcast_2
      (`self.TeleportObject` OtherComp))))

(event `self.Open_Door`
  (`self.ChangeActivity` true)
  (for _array_element (`PrimitiveComponent.GetOverlappingActors` (`self.TeleporterCollider`) null)
    (bind _successfulcast (`self.CastObjectToAcceptableOverlapClasses` _array_element))
    (if _successfulcast
      (`self.TeleportObject` _array_element))))

(event `self.Close_Door`
  (`self.ChangeActivity` false))

(fn `CastObjectToAcceptableOverlapClasses`
  (params (Object :type "Object Object Reference"))
  (returns (SuccessfulCast :type Boolean))
  (locals (ActorPassesCast :type Boolean))
  (set `local.ActorPassesCast` false)
  (for _array_element (`self.AcceptableOverlapClasses`)
    (if (`KismetMathLibrary.ClassIsChildOf` (`GameplayStatics.GetObjectClass` Object) _array_element)
      (set `local.ActorPassesCast` true)
      (break)))
  (return (`local.ActorPassesCast`)))

(fn `ChangeActivity`
  (params (SetActive :type Boolean))
  (`ActorComponent.SetActive` (`self.TeleporterCollider`) SetActive false)
  (`SceneComponent.SetVisibility` (`self.Teleporter`) SetActive false)
  (set `self.TeleporterIsActive` SetActive))

(fn `TeleportObject`
  (params (Object :type "Object Object Reference"))
  (bind _returnvalue (`SceneComponent.K2_GetComponentLocation` (`Actor.RootComponent` (`self.TeleporterExit`))))
  (if (`self.TeleporterIsActive`)
    (bind _asactor (cast `Actor` Object)
      (:`then`
        (`self.K2_TeleportTo` :`self` _asactor :`DestLocation` _returnvalue))
      (:`CastFailed`
        (bind _asstatic_mesh_component (cast `StaticMeshComponent` Object))
        (`SceneComponent.K2_SetWorldLocation` _asstatic_mesh_component _returnvalue false false)))))

(fn `UserConstructionScript`
  (`parent.UserConstructionScript`))