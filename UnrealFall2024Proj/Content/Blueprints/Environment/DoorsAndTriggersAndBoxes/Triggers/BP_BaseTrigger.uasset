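; Base trigger Blueprint that activates linked doors while an allowed actor stands inside its collider.
; Overlap begin and end events check the actor's class, including subclasses, against a list of acceptable classes.
; A passing actor adds or removes active triggers on every door in a map, passing each door its mapped value.
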(event `self.TriggerCollider.OnComponentBeginOverlap`
  (params (OverlappedComponent :type "PrimitiveComponent Object Reference") (OtherActor :type "Actor Object Reference") (OtherComp :type "PrimitiveComponent Object Reference") (OtherBodyIndex :type Integer) (bFromSweep :type Boolean) (SweepResult :type "HitResult Structure (by ref)"))
  (bind _successfulcast (`self.CastActorToAcceptableOverlapClasses` OtherActor))
  (if _successfulcast
    (`self.AddOrRemoveTriggersToCorrespondingDoors` true)))

(event `self.TriggerCollider.OnComponentEndOverlap`
  (params (OverlappedComponent :type "PrimitiveComponent Object Reference") (OtherActor :type "Actor Object Reference") (OtherComp :type "PrimitiveComponent Object Reference") (OtherBodyIndex :type Integer))
  (bind _successfulcast (`self.CastActorToAcceptableOverlapClasses` OtherActor))
  (if _successfulcast
    (`self.AddOrRemoveTriggersToCorrespondingDoors` false)))

(fn `AddOrRemoveTriggersToCorrespondingDoors`
  (params (Add :type Boolean))
  (bind _correspondingdoorstemp (`self.CorrespondingDoorsTemp`))
  (bind _keys (`BlueprintMapLibrary.Map_Keys` _correspondingdoorstemp))
  (for _array_element _keys
    (if Add
      (bind _value (`BlueprintMapLibrary.Map_Find` _correspondingdoorstemp _array_element))
      (`/Game/Blueprints/Environment/DoorsAndTriggersAndBoxes/TriggerDoors/BP_BaseTriggerDoor.AddActiveTriggers` _array_element _value)
      (else
        (`/Game/Blueprints/Environment/DoorsAndTriggersAndBoxes/TriggerDoors/BP_BaseTriggerDoor.RemoveActiveTriggers` _array_element _value)))))

(fn `CastActorToAcceptableOverlapClasses`
  (params (Actor :type "Actor Object Reference"))
  (returns (SuccessfulCast :type Boolean))
  (locals (ActorPassesCast :type Boolean :default false))
  (set `local.ActorPassesCast` false)
  (for _array_element (`self.AcceptableOverlapClasses`)
    (if (`KismetMathLibrary.ClassIsChildOf` (`GameplayStatics.GetObjectClass` Actor) _array_element)
      (set `local.ActorPassesCast` true)
      (break)))
  (return (`local.ActorPassesCast`)))

(fn `UserConstructionScript`)