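; Environment actor that smoothly rotates its FanMiddle component around the yaw axis, apparently a fan.
; Each Tick passes through a Delay of TimeBetweenTicks, then captures the current yaw and restarts the Rotate timeline.
; The timeline's RotationPattern01 curve, scaled by DegreeOfRotation, is added to that starting yaw, while pitch and roll are set to zero.
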(event `self.ReceiveTick`
  (params (DeltaSeconds :type "Float (single-precision)"))
  (bind (_relativerotation_roll _relativerotation_pitch _relativerotation_yaw) (`KismetMathLibrary.BreakRotator` (`SceneComponent.RelativeRotation` (`self.Fan_Middle`))))
  (`KismetSystemLibrary.Delay` (`self.TimeBetweenTicks`))
  (set `self.Current_Rotation` _relativerotation_yaw)
  (bind (_direction _rotationpattern_01) (`Timeline|Rotate` :!via `PlayFromStart`)
    (:`Update`
      (`SceneComponent.K2_SetRelativeRotation` (`self.Fan_Middle`) (`KismetMathLibrary.MakeRotator` 0.0 0.0 (+ (* _rotationpattern_01 (`self.DegreeOfRotation`)) (`self.Current_Rotation`))) false false))))

(fn `UserConstructionScript`)