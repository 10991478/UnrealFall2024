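; Rotating environment obstacle that turns smoothly about its roll axis in repeated steps.
; Tick feeds a Delay of TimeBetweenTicks, which then stores the current roll of ParentTransform and restarts the Rotate timeline.
; The timeline's RotationPattern01 curve, scaled by DegreeOfRotation, is added to that stored roll on each update, with pitch and yaw set from Zero.
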(event `self.ReceiveTick`
  (params (DeltaSeconds :type "Float (single-precision)"))
  (bind _zero (`self.Zero`))
  (bind _relativerotation_roll (`KismetMathLibrary.BreakRotator` (`SceneComponent.RelativeRotation` (`self.ParentTransform`))))
  (`KismetSystemLibrary.Delay` (`self.TimeBetweenTicks`))
  (set `self.Current_Rotation` _relativerotation_roll)
  (bind (_direction _rotationpattern_01) (`Timeline|Rotate` :!via `PlayFromStart`)
    (:`Update`
      (`SceneComponent.K2_SetRelativeRotation` (`self.ParentTransform`) (`KismetMathLibrary.MakeRotator` (+ (* _rotationpattern_01 (`self.DegreeOfRotation`)) (`self.Current_Rotation`)) _zero _zero) false false))))

(fn `UserConstructionScript`)