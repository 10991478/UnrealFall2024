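; BP_RotatingObject_01_Linear_Rotation_Asian_01 is a rotating environment obstacle that turns a wooden beam mesh around its yaw axis in timed steps.
; Tick feeds a Delay of TimeBetweenTicks, which then stores the beam's current yaw and restarts the Rotate timeline.
; The timeline's RotationPattern01 curve, scaled by DegreeOfRotation, is added to the stored yaw, so each step continues from the last angle.
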(event `self.ReceiveTick`
  (params (DeltaSeconds :type "Float (single-precision)"))
  (bind (_relativerotation_roll _relativerotation_pitch _relativerotation_yaw) (`KismetMathLibrary.BreakRotator` (`SceneComponent.RelativeRotation` (`self.SM_wooden_beam_01`))))
  (`KismetSystemLibrary.Delay` (`self.TimeBetweenTicks`))
  (set `self.Current_Rotation` _relativerotation_yaw)
  (bind (_direction _rotationpattern_01) (`Timeline|Rotate` :!via `PlayFromStart`)
    (:`Update`
      (`SceneComponent.K2_SetRelativeRotation` (`self.SM_wooden_beam_01`) (`KismetMathLibrary.MakeRotator` 0.0 0.0 (+ (* _rotationpattern_01 (`self.DegreeOfRotation`)) (`self.Current_Rotation`))) false false))))

(fn `UserConstructionScript`)