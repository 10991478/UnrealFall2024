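; Base checkpoint actor that registers itself and its spawn point location with the third-person character when that character overlaps its collider.
; On BeginPlay it binds to the player character's current-checkpoint broadcast and compares the broadcast ID with its own CheckpointID.
; A match calls ActivateCheckpoint and any other ID calls DeactivateCheckpoint, both empty events in this base.
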(event `self.ReceiveBeginPlay`
  (bind _asbp_third_person_character (cast `/Game/ThirdPerson/Blueprints/BP_ThirdPersonCharacter` (`Controller.K2_GetPawn` (`GameplayStatics.GetPlayerController` 0))))
  (add `/Game/ThirdPerson/Blueprints/BP_ThirdPersonCharacter.ED_BroadcastCurrentCheckpoint` _asbp_third_person_character (delegate `CompareToBroadcastedCheckpoint`)))

(event `CompareToBroadcastedCheckpoint`
  (params (CurrentCheckpointID :type String))
  (if (`KismetStringLibrary.EqualEqual_StrStr` CurrentCheckpointID (`self.CheckpointID`))
    (`self.ActivateCheckpoint`)
    (else
      (`self.DeactivateCheckpoint`))))

(event `self.CheckpointCollider.OnComponentBeginOverlap`
  (params (OverlappedComponent :type "PrimitiveComponent Object Reference") (OtherActor :type "Actor Object Reference") (OtherComp :type "PrimitiveComponent Object Reference") (OtherBodyIndex :type Integer) (bFromSweep :type Boolean) (SweepResult :type "HitResult Structure (by ref)"))
  (bind _asbp_third_person_character (cast `/Game/ThirdPerson/Blueprints/BP_ThirdPersonCharacter` OtherActor))
  (`/Game/ThirdPerson/Blueprints/BP_ThirdPersonCharacter.SetCheckpoint` _asbp_third_person_character (`SceneComponent.K2_GetComponentLocation` (`self.SpawnPoint`)) self))

(event `ActivateCheckpoint`)

(event `DeactivateCheckpoint`)

(fn `UserConstructionScript`)