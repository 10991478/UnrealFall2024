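; Lamp post checkpoint Blueprint that signals its active state with two point lights.
; Both lights are hidden at BeginPlay, after the parent's BeginPlay runs.
; The ActivateCheckpoint and DeactivateCheckpoint events show or hide both lights and print a debug string for the new state.
; The file contains no trigger or respawn logic, only this visual response.
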(event `self.ReceiveBeginPlay`
  (`parent.ReceiveBeginPlay`)
  (`SceneComponent.SetVisibility` (`self.PointLight_01`) false false)
  (`SceneComponent.SetVisibility` (`self.PointLight_02`) false false))

(event `self.ActivateCheckpoint`
  (`SceneComponent.SetVisibility` (`self.PointLight_01`) true false)
  (`SceneComponent.SetVisibility` (`self.PointLight_02`) true false)
  (`KismetSystemLibrary.PrintString` "Activated"))

(event `self.DeactivateCheckpoint`
  (`SceneComponent.SetVisibility` (`self.PointLight_01`) false false)
  (`SceneComponent.SetVisibility` (`self.PointLight_02`) false false)
  (`KismetSystemLibrary.PrintString` "Deactivated"))

(fn `UserConstructionScript`
  (`parent.UserConstructionScript`))